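; PlayerBP is a per-player cursor actor that, on Tick, reads the gamepad matching its PlayerID and sets Movement from the left stick, scaled by PlayerManager power.
; In one state, the right face button claims an overlapped "leaking person", advances state and dims the cursor.
; In another, edge-detected face-button presses increment CCButtomNum unless the player has lost; losers accumulate LoserCount.
; Number keys toggle WASD debug movement per player.
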(event EventBeginPlay)

(event Collision|EventActorBeginOverlap
  (params (OtherActor :type Actor%20Object%20Reference)))

(event EventTick
  (params (DeltaSeconds :type Float%20%28single-precision%29))
  (CallFunction|PlayerMove)
  (CallFunction|GetBottominCC)
  (CallFunction|CatchLeaking)
  (if (Variables|CloseContest|GetLoser)
    (Math|Integer|IncrementInt (Variables|CloseContest|GetLoserCount)
      (:%20%20
        _)))
  ;[1 1 1] Debugメニュー
  (if (Variables|Debug|GetDebug)
    (Variables|Status|SetMovement (* (Variables|Debug|GetDebugMove) (Variables|/Game/Assets/Manager/PlayerManager.PlayerManager_C|GetPower (Variables|Default|GetPlayerManagerRef))))))

(event Input|KeyboardEvents|S
  (params (Key :type Key%20Structure :default "None"))
  ;[1 1 1] デバッグ用
  (:Pressed
    (Variables|Debug|SetDebugMove (Math|Vector2D|MakeVector2D (.X (Math|Vector2D|BreakVector2D (Variables|Debug|GetDebugMove))) 1.0)))
  (:Released
    (Variables|Debug|SetDebugMove (Math|Vector2D|MakeVector2D (.X (Math|Vector2D|BreakVector2D (Variables|Debug|GetDebugMove))) 0.0))))

(event Input|KeyboardEvents|D
  (params (Key :type Key%20Structure :default "None"))
  ;[1 1 1] デバッグ用
  (:Pressed
    (Variables|Debug|SetDebugMove (Math|Vector2D|MakeVector2D 1.0 (.Y (Math|Vector2D|BreakVector2D (Variables|Debug|GetDebugMove))))))
  (:Released
    (Variables|Debug|SetDebugMove (Math|Vector2D|MakeVector2D 0.0 (.Y (Math|Vector2D|BreakVector2D (Variables|Debug|GetDebugMove)))))))

(event Input|KeyboardEvents|1
  (params (Key :type Key%20Structure :default "None"))
  ;[1 1 1] デバッグ用
  (:Pressed
    (if (== (Variables|Status|GetPlayerID) 0)
      (Variables|Debug|SetDebug (not (Variables|Debug|GetDebug))))))

(event Input|KeyboardEvents|2
  (params (Key :type Key%20Structure :default "None"))
  ;[1 1 1] デバッグ用
  (:Pressed
    (if (== (Variables|Status|GetPlayerID) 1)
      (Variables|Debug|SetDebug (not (Variables|Debug|GetDebug))))))

(event Input|KeyboardEvents|3
  (params (Key :type Key%20Structure :default "None"))
  ;[1 1 1] デバッグ用
  (:Pressed
    (if (== (Variables|Status|GetPlayerID) 2)
      (Variables|Debug|SetDebug (not (Variables|Debug|GetDebug))))))

(event Input|KeyboardEvents|4
  (params (Key :type Key%20Structure :default "None"))
  ;[1 1 1] デバッグ用
  (:Pressed
    (if (== (Variables|Status|GetPlayerID) 3)
      (Variables|Debug|SetDebug (not (Variables|Debug|GetDebug))))))

(event Input|KeyboardEvents|W
  (params (Key :type Key%20Structure :default "None"))
  ;[1 1 1] デバッグ用
  (:Pressed
    (Variables|Debug|SetDebugMove (Math|Vector2D|MakeVector2D (.X (Math|Vector2D|BreakVector2D (Variables|Debug|GetDebugMove))) -1.0)))
  (:Released
    (Variables|Debug|SetDebugMove (Math|Vector2D|MakeVector2D (.X (Math|Vector2D|BreakVector2D (Variables|Debug|GetDebugMove))) 0.0))))

(event Input|KeyboardEvents|A
  (params (Key :type Key%20Structure :default "None"))
  ;[1 1 1] デバッグ用
  (:Pressed
    (Variables|Debug|SetDebugMove (Math|Vector2D|MakeVector2D -1.0 (.Y (Math|Vector2D|BreakVector2D (Variables|Debug|GetDebugMove))))))
  (:Released
    (Variables|Debug|SetDebugMove (Math|Vector2D|MakeVector2D 0.0 (.Y (Math|Vector2D|BreakVector2D (Variables|Debug|GetDebugMove)))))))

(fn ConstructionScript)

(fn GetBottominCC
  (if (and (Utilities|Enum|Equal(Enum) (Variables|Status|GetState) "NewEnumerator2") (Math|Boolean|Equal(Boolean) (Variables|CloseContest|GetLoser) false))
    (CallFunction|CCCountPlus (Game|Player|IsInputKeyDown (Game|GetPlayerController (Variables|Status|GetPlayerID)) "Gamepad_FaceButton_Bottom") (Utilities|Array|Get(acopy) (Variables|CloseContest|GetOldKeyStates)))
    (CallFunction|CCCountPlus (Game|Player|IsInputKeyDown (Game|GetPlayerController (Variables|Status|GetPlayerID)) "Gamepad_FaceButton_Right") (Utilities|Array|Get(acopy) (Variables|CloseContest|GetOldKeyStates) 1) 1)
    (CallFunction|CCCountPlus (Game|Player|IsInputKeyDown (Game|GetPlayerController (Variables|Status|GetPlayerID)) "Gamepad_FaceButton_Left") (Utilities|Array|Get(acopy) (Variables|CloseContest|GetOldKeyStates) 2) 2)
    (CallFunction|CCCountPlus (Game|Player|IsInputKeyDown (Game|GetPlayerController (Variables|Status|GetPlayerID)) "Gamepad_FaceButton_Top") (Utilities|Array|Get(acopy) (Variables|CloseContest|GetOldKeyStates) 3) 3)))

(fn CCCountPlus
  (params (NowKey :type Boolean) (OldKey :type Boolean) (index :type Integer))
  (bind (_triggerstate _oldkey) (CallFunction|GamePadTrigger NowKey OldKey))
  (Utilities|Array|SetArrayElem (Variables|CloseContest|GetOldKeyStates) index _oldkey)
  (if _triggerstate
    (bind _result (Math|Integer|IncrementInt (Variables|CloseContest|GetCCButtomNum)))))

(fn PlayerMove
  (bind _playermanagerref (Variables|Default|GetPlayerManagerRef))
  (bind _playerid (Variables|Status|GetPlayerID))
  (bind _returnvalue (Game|GetPlayerController _playerid))
  (bind _power (Variables|/Game/Assets/Manager/PlayerManager.PlayerManager_C|GetPower _playermanagerref))
  (bind (_stickx _sticky) (Class|PlayerController|GetInputAnalogStickState _returnvalue "CAS_LeftStick"))
  (Variables|Status|SetMovement (Math|Vector2D|MakeVector2D (* _stickx _power) (* _sticky (* _power -1.0)))))

(fn CatchLeaking
  (if (and (Utilities|Enum|Equal(Enum) (Variables|Status|GetState) "NewEnumerator0") (Variables|Status|GetIsHitLeaking))
    (if (Game|Player|IsInputKeyDown (Game|GetPlayerController (Variables|Status|GetPlayerID)) "Gamepad_FaceButton_Right")
      (bind _asgame_instance_for_fcx (Utilities|Casting|CastToGameInstanceForFCX (Game|GetGameInstance)))
      (Default|SetSelectMine (.PersonData (Default|GetLeakingPerson (Variables|/Game/Assets/GameInstance/GameInstanceForFCX.GameInstanceForFCX_C|GetLeakingPersonManager _asgame_instance_for_fcx) (Variables|Status|GetHitLeakingID))) (Variables|Status|GetPlayerID))
      (Variables|Status|SetState "NewEnumerator1")
      (Default|PlayerCursorOpacityChange (Variables|Default|GetPlayerManagerRef) (Variables|Status|GetPlayerID) 0.25)
      (Default|HitListAllClearinPlayer (Variables|Default|GetPlayerManagerRef) (Variables|Status|GetPlayerID)))))