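; MapRulerBP is an actor that builds a grid map at BeginPlay by spawning actors from its MapChip array.
; SpawnMapChip passes each row's ten entries to SpawnMapChipProcess, which scales grid indices by Movement and increments Counter per chip.
; SpawnStaticMesh spawns each entry's class at that offset from the ruler's location.
; The first entry in each row has X and Y swapped relative to the other nine.
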(event EventBeginPlay
  (CallFunction|SpawnMapChip))

(event Collision|EventActorBeginOverlap
  (params (OtherActor :type Actor%20Object%20Reference)))

(event EventTick
  (params (DeltaSeconds :type Float%20%28single-precision%29)))

(fn ConstructionScript)

(fn SpawnStaticMesh
  (params (NewParam :type Test%20Object%20BP%20Object%20Reference) (Position :type Vector))
  (Game|SpawnActorfromClass (Utilities|GetClass NewParam) (Math|Transform|MakeTransform (+ Position (Transformation|GetActorLocation self)) "0, 0, 0" "1,1,1") "Undefined" 0 0)
  (return))

(fn SpawnMapChip
  (for (_array_element _array_index) (Variables|Default|GetMapChip)
    (bind _output_get (Variables|Default|Setcounter 0))
    (CallFunction|SpawnMapChipProcess (._0 (Utilities|Struct|BreakMapChipColumn _array_element)) _output_get _array_index)
    (CallFunction|SpawnMapChipProcess (._1 (Utilities|Struct|BreakMapChipColumn _array_element)) _array_index (Variables|Default|Getcounter))
    (CallFunction|SpawnMapChipProcess (._2 (Utilities|Struct|BreakMapChipColumn _array_element)) _array_index (Variables|Default|Getcounter))
    (CallFunction|SpawnMapChipProcess (._3 (Utilities|Struct|BreakMapChipColumn _array_element)) _array_index (Variables|Default|Getcounter))
    (CallFunction|SpawnMapChipProcess (._4 (Utilities|Struct|BreakMapChipColumn _array_element)) _array_index (Variables|Default|Getcounter))
    (CallFunction|SpawnMapChipProcess (._5 (Utilities|Struct|BreakMapChipColumn _array_element)) _array_index (Variables|Default|Getcounter))
    (CallFunction|SpawnMapChipProcess (._6 (Utilities|Struct|BreakMapChipColumn _array_element)) _array_index (Variables|Default|Getcounter))
    (CallFunction|SpawnMapChipProcess (._7 (Utilities|Struct|BreakMapChipColumn _array_element)) _array_index (Variables|Default|Getcounter))
    (CallFunction|SpawnMapChipProcess (._8 (Utilities|Struct|BreakMapChipColumn _array_element)) _array_index (Variables|Default|Getcounter))
    (CallFunction|SpawnMapChipProcess (._9 (Utilities|Struct|BreakMapChipColumn _array_element)) _array_index (Variables|Default|Getcounter))))

(fn SpawnMapChipProcess
  (params (NewParam2 :type Test%20Object%20BP%20Object%20Reference) (X :type Integer) (Y :type Integer))
  (CallFunction|SpawnStaticMesh NewParam2 (* (Math|Vector|MakeVector (Math|Conversions|ToFloat(Integer) X) (Math|Conversions|ToFloat(Integer) Y) 0.0) (Variables|Default|Getmovement)))
  (Math|Integer|IncrementInt (Variables|Default|Getcounter)
    (:%20%20
      (return))))